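; Grid-based combat unit actor, configured from its unit type data, with team-colored HP bar and tile marker, hover/selection tint and HP/MP stats.
; A timeline walks it tile by tile along a path, hopping on height changes and broadcasting progress.
; Spell hits change HP immediately to stay in sync, while bar, floating number and hit or death animation wait until the spell animation hits its tile.
; MP refills on combat start/end and turn end.
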(event Custom|ContinueToFollowPath
  (bind _timeline_unitmovement (Variables|Default|GetTimeline_UnitMovement))
  (bind _grid (Variables|Grid|GetGrid))
  (bind _currentpathtofollow (Variables|UnitMovement|GetCurrentPathToFollow))
  (bind _output (Utilities|Array|Get(acopy) _currentpathtofollow))
  (bind _gridtiles (Variables|/Game/Blueprints/Core/Grid/BP_Grid.BP_Grid_C|GetGridTiles _grid))
  (bind _value (Utilities|Map|Find _gridtiles _output))
  (bind _transform (Utilities|Struct|BreakS_TileData _value))
  ;[0 0 0] [EN] Not done walking? Continue
  ; [FR] Pas terminé de marcher? Continue
  (if (> (Utilities|Array|Length (Variables|UnitMovement|GetCurrentPathToFollow)) 0)
    (Animation|SetAnimationState "NewEnumerator1")
    ;[0 0 0] [EN] Set the current tile and next tile for the interpolation
    ; [FR] Set la case courante et la prochaine case pour l'interpolation
    (Variables|UnitMovement|SetPreviousTransform (Transformation|GetActorTransform))
    (Variables|UnitMovement|SetNextTransform (Math|Transform|MakeTransform (.location _transform) (Math|Rotator|MakeRotator 0.0 0.0 (.yaw (Math|Rotator|FindLookatRotation (.location (Variables|UnitMovement|GetPreviousTransform)) (.location _transform)))) "1,1,1"))
    ;[0 0 0] [EN] Apply desired speed to the timeline
    ; [FR] Appliquer la vitesse voulue à la timeline
    (Components|Timeline|SetPlayRate _timeline_unitmovement (/ (Components|Timeline|GetTimelineLength _timeline_unitmovement) (Variables|UnitMovement|GetMoveDurationPerTile)))
    ;[0 0 0] [EN] Move the unit based on the timeline: Interpolate position to next tile. Look at next tile. If there's a height difference, add a little jump on the location.
    ; [FR] Déplace l'unité basé sur la timeline: Interpole la position vers la prochaine case. Regarde la prochaine case. S'il y a une différence de hauteur, ajoute un petit saut à la location.
    (bind (_direction _locationalpha _rotationalpha _jump) (Timeline|Timeline_UnitMovement PlayFromStart)
      (:Update
        (Transformation|SetActorLocationAndRotation (+ (Math|Vector|Lerp(Vector) (.location (Variables|UnitMovement|GetPreviousTransform)) (.location (Variables|UnitMovement|GetNextTransform)) _locationalpha) (Math|Vector|MakeVector 0.0 0.0 (select (Math|Float|NearlyEqual(Float) (.z (.location (Variables|UnitMovement|GetPreviousTransform))) (.z (.location (Variables|UnitMovement|GetNextTransform))) 5.0) 0.0 _jump))) (Math|Rotator|Lerp(Rotator) (.rotation (Variables|UnitMovement|GetPreviousTransform)) (.rotation (Variables|UnitMovement|GetNextTransform)) _rotationalpha true)))
      (:Finished
        ;[0 0 0] [EN] Next tile reached, remove it from the path and do the next loop
        ; [FR] Arrivé sur la case suivante. Enlève là du path et ensuite exécute la prochaine loop
        (Default|CallOnUnitReachedNewTile self (Utilities|Array|Get(acopy) (Variables|UnitMovement|GetCurrentPathToFollow)))
        (Utilities|Array|RemoveIndex (Variables|UnitMovement|GetCurrentPathToFollow))
        (CallFunction|ContinuetoFollowPath)))
    (else
      ;[0 0 0] [EN] End of the movement
      ; [FR] Fin du mouvement
      (Animation|SetAnimationState "NewEnumerator0")
      (Default|CallOnUnitFinishedWalking self))))

(event Custom|Debug_RespawnAfterFewSeconds
  (Utilities|FlowControl|Delay 2.0)
  (Stats|SetCurrentHp (.HP_Max (Utilities|Struct|BreakS_UnitData_Stats (Utilities|Struct|BreakS_UnitData (Variables|UnitData|GetUnitData)))))
  (Animation|SetAnimationState "NewEnumerator5")
  (Default|EventUpdateHpBar (Variables|UnitData|GetHpBar)))

(event Custom|Event_FollowPath
  (params (Path :type Array%20of%20Int%20Point%20Structures))
  ;[0 0 0] [EN] Beginning of the movement
  ; [FR] Début du mouvement
  (if (> (Utilities|Array|Length Path) 0)
    (Variables|UnitMovement|SetCurrentPathToFollow Path)
    (Default|CallOnUnitStartedWalking self)
    (CallFunction|ContinuetoFollowPath)))

(event EventBeginPlay
  (Animation|SetAnimationState "NewEnumerator0")
  (bind _output_get (Variables|UnitData|SetHpBar (.AsW%20Hp%20Bar (Utilities|Casting|CastToW_HpBar (UserInterface|GetUserWidgetObject (Variables|Default|GetWidget_HpBar))))))
  (Default|EventSetUnit _output_get self))

(fn ConstructionScript
  (bind _unitdata (CallFunction|GetDefaultUnitDatafromUnitType (Variables|UnitData|GetUnitType)))
  (UnitData|SetUnitData _unitdata))

(fn UpdateVisualifHoveredorSelected
  (Rendering|Material|SetVectorParameterValueonMaterials (Variables|Default|GetSkeletalMesh) "ColorMultiply" (Math|Conversions|ToVector(LinearColor) (* (* (select (Variables|Hovered&Selected|GetIsSelected) "(R=0.176490,G=0.523803,B=1.000000,A=1.000000)" "(R=1.000000,G=1.000000,B=1.000000,A=1.000000)") (select (Variables|Hovered&Selected|GetIsHovered) 2.5 1.0)) (select (Variables|Hovered&Selected|GetIsSelected) 2.5 1.0)))))

(fn SetIsHovered
  (params (Hovered :type Boolean))
  (Variables|Hovered&Selected|SetIsHovered Hovered)
  (Hovered&Selected|UpdateVisualifHoveredorSelected)
  (Default|CallOnUnitHoveredChanged self))

(fn SetIsSelected
  (params (Selected :type Boolean))
  (Variables|Hovered&Selected|SetIsSelected Selected)
  (Hovered&Selected|UpdateVisualifHoveredorSelected)
  (Default|CallOnUnitSelectedChanged self))

(fn SetUnitData
  (params (Data :type S%20Unit%20Data%20Structure%20%28by%20ref%29))
  (bind _skeletalmesh (Variables|Default|GetSkeletalMesh))
  (bind _output_get (Variables|UnitData|SetUnitData Data))
  (Class|SkinnedMeshComponent|SetSkeletalMesh _skeletalmesh (.Mesh (Utilities|Struct|BreakS_UnitData_Assets (.Assets (Utilities|Struct|BreakS_UnitData _output_get)))) true)
  (Class|SkeletalMeshComponent|SetAnimClass _skeletalmesh (.AnimBp (Utilities|Struct|BreakS_UnitData_Assets (.Assets (Utilities|Struct|BreakS_UnitData _output_get))))))

(fn GetAnimationState
  (bind _state (Class|BPIUnitAnimation|GetUnitAnimationState(Message) (Components|SkeletalMesh|GetAnimInstance (Variables|Default|GetSkeletalMesh))))
  (return _state))

(fn SetAnimationState
  (params (State :type E_UnitAnimationState%20Enum :default "NewEnumerator0"))
  (Class|BPIUnitAnimation|SetUnitAnimationState(Message) (Components|SkeletalMesh|GetAnimInstance (Variables|Default|GetSkeletalMesh)) State))

(fn SetGrid
  (params (Grid :type BP%20Grid%20Object%20Reference))
  (bind _mesh_teamindex (Variables|Default|GetMesh_TeamIndex))
  (bind _collision_lineofsight (Variables|Default|GetCollision_LineOfSight))
  (Variables|Grid|SetGrid Grid)
  ;[0 0 0] [EN] Setup the collision component so its rotation and scale are behaving properly in game
  ; [FR] Mettre en place le collision component pour qu'il tourne et scale comme on veut
  (Components|StaticMesh|SetStaticMesh _collision_lineofsight (.Mesh (Utilities|Struct|BreakS_GridShapeData (Default|GetCurrentShapeData (Variables|Grid|GetGrid)))))
  (Transformation|SetAbsolute _collision_lineofsight false true true)
  (Transformation|SetWorldScale3D _collision_lineofsight (Math|Vector|MakeVector (.x (/ (Variables|/Game/Blueprints/Core/Grid/BP_Grid.BP_Grid_C|GetGridTileSize (Variables|Grid|GetGrid)) (.MeshSize (Utilities|Struct|BreakS_GridShapeData (Default|GetCurrentShapeData (Variables|Grid|GetGrid)))))) (.y (/ (Variables|/Game/Blueprints/Core/Grid/BP_Grid.BP_Grid_C|GetGridTileSize (Variables|Grid|GetGrid)) (.MeshSize (Utilities|Struct|BreakS_GridShapeData (Default|GetCurrentShapeData (Variables|Grid|GetGrid)))))) (.z (Transformation|GetWorldScale (Variables|Default|GetCollision_LineOfSight)))))
  (Transformation|SetWorldRotation _collision_lineofsight (Default|GetTileRotationfromGridIndex (Variables|Grid|GetGrid) (Variables|UnitData|GetIndex)) false false)
  ;[0 0 0] [EN] Setup the mesh component so its rotation and scale are behaving properly in game. And also adjust the material
  ; [FR] Mettre en place le mesh component pour qu'il tourne et scale comme on veut. Et aussi  on ajuste le materiel
  (Components|StaticMesh|SetStaticMesh _mesh_teamindex (.FlatMesh (Utilities|Struct|BreakS_GridShapeData (Default|GetCurrentShapeData (Variables|Grid|GetGrid)))))
  (Rendering|Material|SetMaterial _mesh_teamindex 0 (.FlatMaterial (Utilities|Struct|BreakS_GridShapeData (Default|GetCurrentShapeData (Variables|Grid|GetGrid)))))
  (Rendering|Material|SetScalarParameterValueonMaterials _mesh_teamindex "IsFilled" 1.0)
  (Transformation|SetAbsolute _mesh_teamindex false true true)
  (Transformation|SetWorldScale3D _mesh_teamindex (/ (Variables|/Game/Blueprints/Core/Grid/BP_Grid.BP_Grid_C|GetGridTileSize (Variables|Grid|GetGrid)) (.MeshSize (Utilities|Struct|BreakS_GridShapeData (Default|GetCurrentShapeData (Variables|Grid|GetGrid))))))
  (Transformation|SetWorldRotation _mesh_teamindex (Default|GetTileRotationfromGridIndex (Variables|Grid|GetGrid) (Variables|UnitData|GetIndex)) false false)
  (Transformation|SetRelativeLocation _mesh_teamindex (Math|Vector|MakeVector 0.0 0.0 (+ (Variables|/Game/Blueprints/Core/Grid/BP_GridVisual.BP_GridVisual_C|GetOffsetFromGround (Variables|/Game/Blueprints/Core/Grid/BP_Grid.BP_Grid_C|GetGridVisual (Variables|Grid|GetGrid))) 5.0)) false false))

(fn SetGridIndex
  (params (Index :type Int%20Point%20Structure))
  (Variables|UnitData|SetIndex Index)
  (Transformation|SetWorldRotation (Variables|Default|GetCollision_LineOfSight) (Default|GetTileRotationfromGridIndex (Variables|Grid|GetGrid) (Variables|UnitData|GetIndex)) false false))

(fn UnitCastSpell
  (params (TargetIndex :type Int%20Point%20Structure%20%28by%20ref%29))
  (bind _returnvalue (Transformation|GetActorLocation))
  (bind _grid (Variables|Grid|GetGrid))
  (bind (_x _y) (Math|Vector|BreakVector _returnvalue))
  (bind _gridtiles (Variables|/Game/Blueprints/Core/Grid/BP_Grid.BP_Grid_C|GetGridTiles _grid))
  (bind _value (Utilities|Map|Find _gridtiles TargetIndex))
  (bind _transform (Utilities|Struct|BreakS_TileData _value))
  (bind (_x_2 _y_2) (Math|Vector|BreakVector (.location _transform)))
  ;[0 0 0] [EN] Look at the target then play the attack animation
  ; [FR] Regarde la cible et ensuite joue l'animation d'attaque
  (Transformation|SetActorRotation (Math|Rotator|FindLookatRotation (Math|Vector|MakeVector _x _y 0.0) (Math|Vector|MakeVector _x_2 _y_2 0.0)))
  (Animation|SetAnimationState "NewEnumerator2"))

(fn UnitHitbySpell
  (params (SpellImpactReal :type S%20Spell%20Data%20Impact%20Real%20Structure) (SpellAnimation :type BP%20Spell%20Animation%20Object%20Reference))
  (bind _modifier_hp (Utilities|Struct|BreakS_SpellData_Impact_Real SpellImpactReal))
  ;[0 0 0] [EN] Get ready to play the animations. For timing purposes
  ; [FR] Se préparer à jouer l'animation. Dans le but d'alligner les timings
  (Utilities|Map|Add (Variables|Spells|GetIncomingSpellImpacts) SpellAnimation SpellImpactReal)
  (EventDispatchers|BindEventtoOnSpellAnimationHitTile SpellAnimation (EventDispatchers|CreateEvent :!event OnSpellAnimationHitTile))
  ;[0 0 0] [EN] But modify the unit stats right away so we're never out of sync
  ; [FR] Mais on modifie les stats de l'unité immédiatement pour ne pas qu'on soit désyncronisé
  (if (!= _modifier_hp 0) ; Modifying Hp?
    (Stats|ModifyCurrentHp _modifier_hp)))

(fn ModifyCurrentHp
  (params (Modifier :type Integer))
  (Stats|SetCurrentHp (+ Modifier (.HP_Current (Utilities|Struct|BreakS_UnitData_Stats (Utilities|Struct|BreakS_UnitData (Variables|UnitData|GetUnitData)))))))

(fn SetCurrentHp
  (params (Hp :type Integer))
  (bind _structout (Utilities|Struct|SetmembersinS_UnitData_Stats (Utilities|Struct|BreakS_UnitData (Variables|UnitData|GetUnitData)) (Math|Integer|Clamp(Integer) Hp 0 (.HP_Max (Utilities|Struct|BreakS_UnitData_Stats (Utilities|Struct|BreakS_UnitData (Variables|UnitData|GetUnitData)))))))
  (Utilities|Struct|SetmembersinS_UnitData (Variables|UnitData|GetUnitData) _structout))

(fn OnSpellAnimationHitTile
  (params (SpellAnimation :type BP%20Spell%20Animation%20Object%20Reference) (TileIndex :type Int%20Point%20Structure))
  (bind _incomingspellimpacts (Variables|Spells|GetIncomingSpellImpacts))
  (bind (_value _returnvalue) (Utilities|Map|Find _incomingspellimpacts SpellAnimation))
  ;[0 0 0] [EN] Do we process this spell?
  ; [FR] Est-ce qu'on applique ce sort?
  (if (Class|KismetMathLibrary|EqualIntPointIntPoint (Variables|UnitData|GetIndex) TileIndex) ; Is this my tile?
    (if _returnvalue ; Do I still need to process this spell?
      (LocalVariables|SetSpellImpactReal _value)
      (Utilities|Map|Remove (Variables|Spells|GetIncomingSpellImpacts) SpellAnimation)
      ;[0 0 0] [EN] If it's a spell that affects the HP, we update the hp bar and spawn the AnimatedNumber. If this is a damaging spell, we either ask the unit to play its hit animation or its death animation depending if it's alive or not
      ; [FR] Si c'est un sort qui affecte les HP, on met à jour la barre de vie et spawn le AnimatedNumber. S'il s'agit d'un sort qui fait du domage, on demande à l'unité de jouer son hit animation. Ou alors son death animation s'il est mort
      (if (!= (Utilities|Struct|BreakS_SpellData_Impact_Real (LocalVariables|GetSpellImpactReal)) 0)
        (Default|EventUpdateHpBar (Variables|UnitData|GetHpBar))
        (Game|SpawnActorfromClass "/Game/Blueprints/Core/Units/Widgets/BP_AnimatedNumber.BP_AnimatedNumber_C" (Math|Transform|MakeTransform (Transformation|GetActorLocation) "0, 0, 0" "1,1,1") "Undefined" 0 (Utilities|Struct|BreakS_SpellData_Impact_Real (LocalVariables|GetSpellImpactReal)) "NewEnumerator0" 0)
        (if (< (Utilities|Struct|BreakS_SpellData_Impact_Real (LocalVariables|GetSpellImpactReal)) 0) ; Damaged the Unit?
          (if (== (.HP_Current (Utilities|Struct|BreakS_UnitData_Stats (Utilities|Struct|BreakS_UnitData (Variables|UnitData|GetUnitData)))) 0) ; Is it dead?
            (if (Utilities|Enum|NotEqual(Enum) (Animation|GetAnimationState) "NewEnumerator4")
              (Animation|SetAnimationState "NewEnumerator4"))
            (else
              (Animation|SetAnimationState "NewEnumerator3"))))))))

(fn SetTeamIndex
  (params (Index :type Integer))
  ;[0 0 0] [EN] We display the team index to the player in 2 ways: Color of the HP bar and color of the tile under the unit
  ; [FR] On affiche l'index de l'équipe au joueur de 2 façons: Couleur de la barre de vie et couleur de la case sous l'unité
  (Variables|Team|SetTeamIndex Index)
  (Class|ProgressBar|SetFillColorandOpacity (Variables|/Game/Blueprints/Core/Units/Widgets/W_HpBar.W_HpBar_C|GetProgressBar_Hp (Variables|UnitData|GetHpBar)) (CallFunction|GetTeamColor (Variables|Team|GetTeamIndex)))
  (Rendering|Material|SetVectorParameterValueonMaterials (Variables|Default|GetMesh_TeamIndex) "Color" (Math|Conversions|ToVector(LinearColor) (CallFunction|GetTeamColor (Variables|Team|GetTeamIndex)))))

(fn CombatStarted
  (Development|PrintString "I'm in combat!")
  ;[0 0 0] [EN] Refill MP at beginning of combat
  ; [FR] Repli les MP au début du combat
  (Stats|ResetMp))

(fn TurnStarted
  (Development|PrintString "It's my turn!"))

(fn TurnEnded
  (Development|PrintString "Sleep time!")
  ;[0 0 0] [EN] Refill MP at end of turn
  ; [FR] Repli les MP à la fin du tour
  (Stats|ResetMp))

(fn CombatEnded
  (Development|PrintString "Vacation time!")
  ;[0 0 0] [EN] Refill MP at end of combat
  ; [FR] Repli les MP à la fin du combat
  (Stats|ResetMp))

(fn ModifyCurrentMp
  (params (Modifier :type Integer) (ShowNumber :type Boolean))
  (Stats|SetCurrentMp (+ Modifier (.MP_Current (Utilities|Struct|BreakS_UnitData_Stats (Utilities|Struct|BreakS_UnitData (Variables|UnitData|GetUnitData))))) ShowNumber))

(fn SetCurrentMp
  (params (Mp :type Integer) (ShowNumber :type Boolean))
  (bind _unitdata (Variables|UnitData|GetUnitData))
  (bind _stats (Utilities|Struct|BreakS_UnitData _unitdata))
  (bind (_mp_current _mp_max) (Utilities|Struct|BreakS_UnitData_Stats _stats))
  (LocalVariables|SetDifference (- Mp _mp_current))
  (bind _structout (Utilities|Struct|SetmembersinS_UnitData_Stats (Utilities|Struct|BreakS_UnitData (Variables|UnitData|GetUnitData)) (Math|Integer|Clamp(Integer) Mp 0 _mp_max)))
  (Utilities|Struct|SetmembersinS_UnitData (Variables|UnitData|GetUnitData) _structout)
  (if (and ShowNumber (!= (LocalVariables|GetDifference) 0))
    (Game|SpawnActorfromClass "/Game/Blueprints/Core/Units/Widgets/BP_AnimatedNumber.BP_AnimatedNumber_C" (Math|Transform|MakeTransform (Transformation|GetActorLocation) "0, 0, 0" "1,1,1") "Undefined" 0 (LocalVariables|GetDifference) "NewEnumerator1" 0)))

(fn ResetMp
  (Stats|SetCurrentMp (Utilities|Struct|BreakS_UnitData_Stats (Utilities|Struct|BreakS_UnitData (Variables|UnitData|GetUnitData))) true))