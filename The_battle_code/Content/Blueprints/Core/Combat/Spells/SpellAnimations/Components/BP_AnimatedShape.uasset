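; BP_AnimatedShape is a spell animation actor that displays a configurable shape travelling from an origin transform to a target transform.
; On BeginPlay it applies the given mesh, material and color, then runs a timeline at the configured play rate.
; The timeline lerps the transform, adding a fixed lift and an animated height offset.
; When finished, it broadcasts OnShapeAnimationCompleted and destroys itself after a short delay.
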(event EventBeginPlay
  (bind _animatedshape (Variables|Default|GetAnimatedShape))
  ;[0 0 0] [EN] Basic blueprint that sets the desired visual and then simply slides from the origin to the target.
  ; [FR] Blueprint de base qui applique le visuel voulu pour ensuite simplement glisser à partir de l'origin vers la target
  (Components|StaticMesh|SetStaticMesh _animatedshape (Variables|Default|GetMesh))
  (Rendering|Material|SetMaterial _animatedshape 0 (Variables|Default|GetMaterial))
  (Rendering|Material|SetVectorParameterValueonMaterials _animatedshape "Color" (Math|Conversions|ToVector(LinearColor) (Variables|Default|GetColor)))
  (Components|Timeline|SetPlayRate (Variables|Default|GetTimeline_PlayAnimation) (Variables|Default|GetPlayRate))
  (bind (_direction _transformalpha _heightoffset) (Timeline|Timeline_PlayAnimation PlayFromStart)
    (:Update
      (Transformation|SetActorTransform (Math|Transform|MakeTransform (+ (.location (Math|Transform|Lerp(Transform) (Variables|Default|GetOriginTransform) (Variables|Default|GetTargetTransform) _transformalpha)) "0, 0,100.000000" (Math|Vector|MakeVector 0.0 0.0 _heightoffset)) (.rotation (Math|Transform|Lerp(Transform) (Variables|Default|GetOriginTransform) (Variables|Default|GetTargetTransform) _transformalpha)) (.scale (Math|Transform|Lerp(Transform) (Variables|Default|GetOriginTransform) (Variables|Default|GetTargetTransform) _transformalpha)))))
    (:Finished
      (Default|CallOnShapeAnimationCompleted self)
      (Utilities|FlowControl|Delay 0.5)
      (Actor|DestroyActor))))

(fn ConstructionScript)