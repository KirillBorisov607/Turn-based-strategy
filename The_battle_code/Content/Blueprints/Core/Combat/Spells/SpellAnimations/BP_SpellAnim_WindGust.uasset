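; BP_SpellAnim_WindGust is the spell animation actor for a wind gust that hits a target tile and spreads to the other attacked tiles.
; After a short delay it reports a hit on the target tile, then spawns a growing BP_AnimatedWindGust from there toward each remaining attacked tile at a random play rate.
; Each gust reports its tile hit when it finishes, and the spell completes once none remain.
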(event Custom|OnShapeAnimationCompletedd
  (params (AnimatedShape :type BP%20Animated%20Wind%20Gust%20Object%20Reference))
  (bind _index (Variables|/Game/Blueprints/Core/Combat/Spells/SpellAnimations/Components/BP_AnimatedWindGust.BP_AnimatedWindGust_C|GetIndex AnimatedShape))
  (bind _attackedindexes (Variables|Default|GetAttackedIndexes))
  (Default|CallOnSpellAnimationHitTile self _index)
  (Utilities|Array|RemoveItem _attackedindexes _index)
  (if (== (Utilities|Array|Length _attackedindexes) 0)
    (CallFunction|EventCompleteSpellAnimation)))

(event EventEventPlaySpellAnimation
  (bind _targetindex (Variables|Default|GetTargetIndex))
  (bind _transform (CallFunction|GetTileTransform _targetindex))
  (Utilities|FlowControl|Delay 0.1)
  (Default|CallOnSpellAnimationHitTile self (Variables|Default|GetTargetIndex))
  (Utilities|Array|RemoveItem (Variables|Default|GetAttackedIndexes) (Variables|Default|GetTargetIndex))
  (for _array_element (Variables|Default|GetAttackedIndexes)
    (bind _returnvalue (Game|SpawnActorfromClass "/Game/Blueprints/Core/Combat/Spells/SpellAnimations/Components/BP_AnimatedWindGust.BP_AnimatedWindGust_C" (Math|Transform|MakeTransform "0, 0, 0" "0, 0, 0" "1,1,1") "AlwaysSpawn" 0 (Math|Transform|MakeTransform (.location _transform) (Math|Rotator|FindLookatRotation (.location _transform) (.location (CallFunction|GetTileTransform _array_element))) "0.500000,0.500000,0.500000") (Math|Transform|MakeTransform (.location (CallFunction|GetTileTransform _array_element)) (Math|Rotator|FindLookatRotation (.location _transform) (.location (CallFunction|GetTileTransform _array_element))) "1.200000,1.200000,1.200000") (Math|Random|RandomFloatinRange 0.8 1.5) _array_element 0))
    (EventDispatchers|AssignOnShapeAnimationCompleted _returnvalue (delegate Custom|OnShapeAnimationCompletedd))))

(fn ConstructionScript
  (|CallParentFunction))