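; BP_OptionsMenu is an options menu actor that shows the menu widget over a rotating streamed-level backdrop.
; On BeginPlay it creates the options widget and adds it to the viewport.
; It then loops endlessly through the Square, Hexagon and Triangle sublevels, streaming each in and out with timed delays while triggering the widget's show and hide background events around each swap.
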(event EventBeginPlay
  (bind _returnvalue (UserInterface|CreateWidget "/Game/Blueprints/Other/MainMenu/W_OptionsMenu.W_OptionsMenu_C"))
  (bind _output_get (Variables|Default|SetW_OptionsMenu _returnvalue))
  (UserInterface|Viewport|AddtoViewport _output_get 0)
  (Game|LoadStreamLevel(byName) "L_Square" true :!label _label)
  (Default|EventShowBackground (Variables|Default|GetW_OptionsMenu))
  (Utilities|FlowControl|Delay 1e+01)
  (Default|EventHideBackground (Variables|Default|GetW_OptionsMenu))
  (Utilities|FlowControl|Delay 5.0)
  (Game|UnloadStreamLevel(byName) "L_Square" false)
  (Game|LoadStreamLevel(byName) "L_Hexagon" true)
  (Default|EventShowBackground (Variables|Default|GetW_OptionsMenu))
  (Utilities|FlowControl|Delay 1e+01)
  (Default|EventHideBackground (Variables|Default|GetW_OptionsMenu))
  (Utilities|FlowControl|Delay 5.0)
  (Game|UnloadStreamLevel(byName) "L_Hexagon" false)
  (Game|LoadStreamLevel(byName) "L_Triangle" true)
  (Default|EventShowBackground (Variables|Default|GetW_OptionsMenu))
  (Utilities|FlowControl|Delay 1e+01)
  (Default|EventHideBackground (Variables|Default|GetW_OptionsMenu))
  (Utilities|FlowControl|Delay 5.0)
  (Game|UnloadStreamLevel(byName) "L_Triangle" false)
  (goto _label))

(fn ConstructionScript)